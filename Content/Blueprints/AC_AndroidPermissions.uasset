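; An actor component that checks and requests Android app permissions at runtime and reports the result through a completion dispatcher.
; RequestPermissions records permissions already granted and requests only the missing ones, finishing immediately if none remain.
; The grant callback appends each result to the status list, while a timeout timer reports failure if it fires first.
; Both paths clear the timer and broadcast success plus per-permission status.
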(event `RequestPermissions`
  (params (AppPermissions :type "Array of String") (TimeoutValue :type "Float (double-precision)"))
  ;[0.2045 0.4034 1 1 40] ANDROID PERMISSIONS
  ;;[1 1 1] Clear any previous data
  (`KismetArrayLibrary.Array_Clear` (`self.PermissionsToRequest`))
  (`KismetArrayLibrary.Array_Clear` (`self.PermissionStatus`))
  ;;[1 1 1] Check if we already have permission for this
  (for _array_element AppPermissions
    (bind _returnvalue (`AndroidPermissionFunctionLibrary.CheckPermission` _array_element))
    (if _returnvalue
      ;;[1 1 1] Add all permissions we already have
      (`KismetArrayLibrary.Array_Add` (`self.PermissionStatus`) (make `/Game/Blueprints/S_PermissionStatus` _array_element true))
      (else
        ;;[1 1 1] Or add it to permissions we need to request
        (`KismetArrayLibrary.Array_Add` (`self.PermissionsToRequest`) _array_element))))
  (if (> (`KismetArrayLibrary.Array_Length` (`self.PermissionsToRequest`)) 0)
    ;;[1 1 1] Request for outstanding permissions
    (bind _returnvalue_2 (`AndroidPermissionFunctionLibrary.AcquirePermissions` (`self.PermissionsToRequest`)))
    (add `AndroidPermissionCallbackProxy.OnPermissionsGrantedDynamicDelegate` _returnvalue_2 (delegate `PermissionsGranted`))
    ;;[1 1 1] Setup the timeout timer
    (bind _returnvalue_3 (`KismetSystemLibrary.K2_SetTimerDelegate` (delegate `PermissionsFailed`) TimeoutValue))
    (set `self.TimeoutTimerHandle` _returnvalue_3)
    (else
      (`self.PermissionsComplete` true))))

(event `PermissionsFailed`
  ;[0.2045 0.4034 1 1 40] ANDROID PERMISSIONS
  ;;[1 1 1] Setup the timeout timer
  (`self.PermissionsComplete` false))

(event `PermissionsGranted`
  (params (Permissions :type "Array of String (by ref)") (GrantResults :type "Array of Boolean (by ref)"))
  ;[0.2045 0.4034 1 1 40] ANDROID PERMISSIONS
  ;;[1 1 1] Collect the result
  (for (_array_element _array_index) Permissions
    (`KismetArrayLibrary.Array_Add` (`self.PermissionStatus`) (make `/Game/Blueprints/S_PermissionStatus` _array_element (`|GetArrayItem` GrantResults _array_index))))
  (`self.PermissionsComplete` true))

(event `PermissionsComplete`
  (params (Success :type Boolean))
  ;[1 1 1] Permission Complete Event
  (`KismetSystemLibrary.K2_ClearAndInvalidateTimerHandle` (`self.TimeoutTimerHandle`))
  (`self.PermissionCompleted` Success (`self.PermissionStatus`)))