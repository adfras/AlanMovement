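; Actor component that drives per-frame skeletal correction logic on an owner that has an Oculus XR body tracking component.
; On BeginPlay or Initialize, it destroys itself if body tracking is missing, otherwise caches and initializes the owner's AC_DeformationLogic and AC_TwistDistribution components.
; Its Tick applies deformation, then twist, so both run in a fixed order from one place, skipping whichever component is absent.
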(event `self.ReceiveBeginPlay`
  (bind _returnvalue (`self.GetOwner`))
  (bind _returnvalue_2 (`Actor.GetComponentByClass` _returnvalue "/Script/OculusXRMovement.OculusXRBodyTrackingComponent"))
  (`|ExecutionSequence` :!label _label
    (:`then_0`
      (`/Engine/EditorBlueprintResources/StandardMacros.IsValid` _returnvalue_2
        (:`Is Valid`
          (set `self.OculusBodyTracking` _returnvalue_2)
          (bind _output_get (set `self.DeformationLogic` (`Actor.GetComponentByClass` _returnvalue "/Game/Blueprints/Deformation/AC_DeformationLogic.AC_DeformationLogic_C")))
          (`/Engine/EditorBlueprintResources/StandardMacros.IsValid` _output_get
            (:`Is Valid`
              (`/Game/Blueprints/Deformation/AC_DeformationLogic.Initialize` _output_get))
            (:`Is Not Valid`
              _))
          (bind _output_get_2 (set `self.TwistDistribution` (`Actor.GetComponentByClass` _returnvalue "/Game/Blueprints/TwistDistriBution/AC_TwistDistribution.AC_TwistDistribution_C")))
          (`/Engine/EditorBlueprintResources/StandardMacros.IsValid` _output_get_2
            (:`Is Valid`
              (`/Game/Blueprints/TwistDistriBution/AC_TwistDistribution.Initialize` _output_get_2))))
        (:`Is Not Valid`
          (`self.K2_DestroyComponent`))))
    (:`then_1`
      (`self.SetComponentTickEnabled` true))))

(event `Initialize`
  (goto _label))

(event `self.ReceiveTick`
  (params (DeltaSeconds :type "Float (single-precision)"))
  (bind _deformationlogic (`self.DeformationLogic`)
    (:`then`
      (`/Game/Blueprints/Deformation/AC_DeformationLogic.ApplyDeformation` _deformationlogic))
    (:`else`
      _))
  (bind _twistdistribution (`self.TwistDistribution`)
    (:`then`
      (`/Game/Blueprints/TwistDistriBution/AC_TwistDistribution.ApplyTwist` _twistdistribution))
    (:`else`)))