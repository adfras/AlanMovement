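; BP_Printer is a debug actor that prints numbered messages into the world as a scrolling stack of TextRender actors.
; Each Print call prefixes a running count, spawns a text actor at the TextSpawnTransform with configured color and size, then shifts all stored lines down.
; CurrentIndex wraps around MaxPrintCount like a ring buffer, so once the limit is passed the actor at that slot is destroyed before the new one is inserted.
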(event `self.ReceiveBeginPlay`)

(event `Print`
  (params (Text :type Text))
  (`self.FormatAndSetText` Text)
  (bind _result (`/Engine/EditorBlueprintResources/StandardMacros.IncrementInt` (`self.TotalPrintCounter`))
    (:`  `
      (if (not (<= _result (`self.MaxPrintCount`)))
        (`self.DeleteItemFromCurrentIndex`))
      (bind _returnvalue (`|SpawnActorFromClass` "/Script/Engine.TextRenderActor" (`SceneComponent.K2_GetComponentToWorld` (`self.TextSpawnTransform`)) "Undefined" "MultiplyWithRoot" null null))
      (`KismetArrayLibrary.Array_Insert` (`self.TextRenderers`) _returnvalue (`self.CurrentIndex`))
      (`self.TextRenderSetup` _returnvalue)
      (`|ExecutionSequence`
        (:`then_0`
          (`self.SetCurrentIndexToNextIndex`))
        (:`then_1`
          (for _array_element (`self.TextRenderers`)
            (bind _returnvalue_2 (`SceneComponent.GetRelativeTransform` (`TextRenderActor.TextRender` _array_element)))
            (`self.K2_SetActorRelativeLocation` _array_element (`KismetMathLibrary.MakeVector` (.x (.location _returnvalue_2)) (.y (.location _returnvalue_2)) (- (.z (.location _returnvalue_2)) 5.0)) false false)))))))

(fn `DeleteItemFromCurrentIndex`
  (bind _output (`|GetArrayItem` (`self.TextRenderers`) (`self.CurrentIndex`)))
  (`/Engine/EditorBlueprintResources/StandardMacros.IsValid` _output
    (:`Is Valid`
      (bind _output_get (set `self.ActorToDelete` _output))
      (`KismetArrayLibrary.Array_RemoveItem` (`self.TextRenderers`) _output_get)
      (`self.K2_DestroyActor` _output_get))))

(fn `FormatAndSetText`
  (params (InText :type "Text (by ref)"))
  (set `self.TextToPrint` (`KismetTextLibrary.Conv_StringToText` (`KismetStringLibrary.Concat_StrStr` (`KismetStringLibrary.Conv_IntToString` (+ (`self.TotalPrintCounter`) 1)) "- " (`KismetTextLibrary.Conv_TextToString` InText)))))

(fn `SetCurrentIndexToNextIndex`
  (set `self.CurrentIndex` (mod (+ (`self.CurrentIndex`) 1) (`self.MaxPrintCount`))))

(fn `TextRenderSetup`
  (params (TextRenderer :type "TextRenderActor Object Reference"))
  (bind _textrender (`TextRenderActor.TextRender` TextRenderer))
  (`TextRenderComponent.SetTextRenderColor` _textrender (`self.TextColor`))
  (`TextRenderComponent.K2_SetText` _textrender (`self.TextToPrint`))
  (`TextRenderComponent.SetWorldSize` _textrender (`self.TextSize`)))

(fn `UserConstructionScript`)