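; Game mode for the Movement SDK Samples that handles Quest render setup, Android permissions and focus-based pausing.
; BeginPlay runs render console commands, then requests device-specific permissions for Quest Pro or Quest 3, including Link, warning on other listed devices.
; Successful grants set a GameInstance flag that skips later requests, while failures print each permission's status.
; Tick pauses the game whenever input focus is lost and resumes it on return.
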(event `self.ReceiveBeginPlay`
  (bind _returnvalue (`OculusXRFunctionLibrary.GetDeviceType`))
  (bind _ac_androidpermissions (`self.AC_AndroidPermissions`))
  ;[1 1 1] Ensure the game looks good on Quest
  (`self.ExecuteCommands` (`self.RenderCommands`) (`GameplayStatics.GetPlayerController` 0))
  ;[1 1 1] Request Android Permissions
  (`KismetSystemLibrary.PrintString` (`KismetStringLibrary.Conv_NameToString` (`HeadMountedDisplayFunctionLibrary.GetHMDDeviceName`)))
  (bind _asbp_game_instance (cast `/Game/Blueprints/BP_GameInstance` (`GameplayStatics.GetGameInstance`)))
  (if (not (`/Game/Blueprints/BP_GameInstance.HaveCheckedForPermissions` _asbp_game_instance))
    (`KismetSystemLibrary.PrintString` (`|GetEnumeratorNameAsString` _returnvalue))
    (switch `EOculusXRDeviceType` _returnvalue
      (:`OculusMobile_Deprecated0`
        (`KismetSystemLibrary.PrintString` "Unsupported device, Movement SDK Samples only support Quest 3 and Quest Pro" true true (struct :`R` 1.0 :`G` 0.234407 :`A` 1.0) 10.0 :!label _label))
      (:`OculusQuest_Deprecated`
        (goto _label))
      (:`OculusQuest2`
        (goto _label))
      (:`MetaQuestPro`
        (set `self.PlatformPermissions` (`self.RequiredPermissionsQuestPro`) :!label _label_2)
        (`/Game/Blueprints/AC_AndroidPermissions.RequestPermissions` _ac_androidpermissions (`self.PlatformPermissions`) 20.0 :!label _label_3)
        (add `/Game/Blueprints/AC_AndroidPermissions.PermissionCompleted` _ac_androidpermissions (delegate `PermissionComplete`)))
      (:`MetaQuest3`
        (set `self.PlatformPermissions` (`self.RequiredPermissionsQuest3`) :!label _label_4)
        (goto _label_3))
      (:`Rift`
        (goto _label))
      (:`Rift_S`
        (goto _label))
      (:`Quest_Link_Deprecated`
        (goto _label))
      (:`Quest2_Link`
        (goto _label))
      (:`MetaQuestProLink`
        (goto _label_2))
      (:`MetaQuest3Link`
        (goto _label_4))
      (:`OculusUnknown`
        (goto _label)))))

(event `PermissionComplete`
  (params (Success :type Boolean) (PermissionStatus :type "Array of /Game/Blueprints/S_PermissionStatus Structure (by ref)"))
  ;[1 1 1] Request Android Permissions
  (if Success
    (set `/Game/Blueprints/BP_GameInstance.HaveCheckedForPermissions` true (stale `self.ReceiveBeginPlay` _asbp_game_instance))
    (else
      ;;[1 0.4466 0.4267] Something is wrong with permissions: Likely is that you have asked for a permission that does not exist on that particular platform / device, or there might be a typo in the permission you are requesting
      (`KismetSystemLibrary.PrintString` "Unable to grant all permissions:" true true (struct :`R` 1.0 :`G` 0.019608 :`A` 1.0) 10.0)
      (for _array_element PermissionStatus
        (bind (_permission _granted) (break `/Game/Blueprints/S_PermissionStatus` _array_element))
        (`KismetSystemLibrary.PrintString` (`KismetStringLibrary.Concat_StrStr` "Permission: " _permission " :: " (`KismetStringLibrary.Conv_BoolToString` _granted)) true true (struct :`R` 1.0 :`G` 0.020172 :`A` 1.0) 10.0)))))

(event `self.ReceiveTick`
  (params (DeltaSeconds :type "Float (single-precision)"))
  (bind _returnvalue (`GameplayStatics.IsGamePaused`))
  (`|ExecutionSequence`
    (:`then_0`
      (if (`OculusXRFunctionLibrary.HasInputFocus`)
        (if _returnvalue
          (`GameplayStatics.SetGamePaused` false))
        (elif (not _returnvalue)
          (`GameplayStatics.SetGamePaused` true))))))

(fn `ExecuteCommands`
  (params (Commands :type "Array of String") (Player :type "PlayerController Object Reference"))
  (for _array_element Commands
    (`KismetSystemLibrary.ExecuteConsoleCommand` _array_element Player)))

(fn `GetFailedPermissions`
  (params (Permissions :type "Map of String to Boolean"))
  (returns (FailedPermissions :type "Array of String"))
  (locals (OutstandingPermissions :type "Array of String"))
  (bind _keys (`BlueprintMapLibrary.Map_Keys` Permissions))
  (for _array_element _keys
    (bind (_value _returnvalue) (`BlueprintMapLibrary.Map_Find` Permissions _array_element))
    (if _returnvalue
      (if (== _value false)
        (`KismetArrayLibrary.Array_AddUnique` (`local.OutstandingPermissions`) _array_element))
      (else
        (`KismetSystemLibrary.PrintString` "Failed to find map value"))))
  (return (`local.OutstandingPermissions`)))

(fn `UserConstructionScript`)