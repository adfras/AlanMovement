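; Oculus VR pawn that lets the player point at and click UMG widgets with tracked hands or motion controllers.
; Each tick it aims both widget interactions from hand pointer poses or controller transforms, placing cursor spheres at hit points over focusable widgets and hiding them on low confidence.
; Index pinches send left mouse clicks and recolor a dynamic material shared by both spheres.
; Local-floor tracking origin is set after a short delay to avoid floor-stuck avatars.
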(event `self.ReceiveBeginPlay`
  (`parent.ReceiveBeginPlay`)
  (bind _returnvalue (`KismetMaterialLibrary.CreateDynamicMaterialInstance` "/Game/Materials/M_Cursor.M_Cursor"))
  (bind _output_get (set `self.SphereMaterial` _returnvalue))
  (`PrimitiveComponent.SetMaterial` (`self.InteractionSphereLeft`) 0 _output_get)
  (`PrimitiveComponent.SetMaterial` (`self.InteractionSphereRight`) 0 _output_get)
  ;[1 1 1] If we set the tracking origin too quickly we might end up with the Avatar stuck in the floor, hence this short delay
  (`KismetSystemLibrary.Delay` 0.2)
  (`HeadMountedDisplayFunctionLibrary.SetTrackingOrigin` "LocalFloor"))

(event `self.ReceiveTick`
  (params (DeltaSeconds :type "Float (single-precision)"))
  (`self.UpdateWidgetInteractions`)
  (`self.UpdateControllers`))

(event `InputAction|IndexPinchLeft`
  (params (Key :type "Key Structure"))
  (bind _spherematerial (`self.SphereMaterial`))
  (bind _widgetinteractionleft (`self.WidgetInteractionLeft`))
  (:`Pressed`
    (`WidgetInteractionComponent.PressPointerKey` _widgetinteractionleft "LeftMouseButton")
    (`MaterialInstanceDynamic.SetVectorParameterValue` _spherematerial "Color" (struct :`R` 0.117468 :`G` 1.0 :`B` 0.12482 :`A` 1.0) :!label _label))
  (:`Released`
    (`WidgetInteractionComponent.ReleasePointerKey` _widgetinteractionleft "LeftMouseButton")
    (`MaterialInstanceDynamic.SetVectorParameterValue` _spherematerial "Color" (struct :`R` 1.0 :`G` 0.316444 :`B` 0.054146 :`A` 1.0) :!label _label_2)))

(event `InputAction|IndexPinchRight`
  (params (Key :type "Key Structure"))
  (bind _widgetinteractionright (`self.WidgetInteractionRight`))
  (:`Pressed`
    (`WidgetInteractionComponent.PressPointerKey` _widgetinteractionright "LeftMouseButton")
    (goto _label))
  (:`Released`
    (`WidgetInteractionComponent.ReleasePointerKey` _widgetinteractionright "LeftMouseButton")
    (goto _label_2)))

(fn `UpdateControllers`
  (`SceneComponent.SetVisibility` (`self.MotionControllerLeft`) (and (not (`OculusXRInputFunctionLibrary.IsHandTrackingEnabled`)) (`self.DisplayControllers`)) true)
  (`SceneComponent.SetVisibility` (`self.MotionControllerRight`) (and (not (`OculusXRInputFunctionLibrary.IsHandTrackingEnabled`)) (`self.DisplayControllers`)) true))

(fn `UpdateWidgetInteractions`
  (bind (_returnvalue_location _returnvalue_rotation) (`KismetMathLibrary.BreakTransform` (`OculusXRInputFunctionLibrary.GetPointerPose` "HandLeft")))
  (bind (_returnvalue_location_2 _returnvalue_rotation_2) (`KismetMathLibrary.BreakTransform` (`OculusXRInputFunctionLibrary.GetPointerPose` "HandRight")))
  (bind _widgetinteractionright (`self.WidgetInteractionRight`))
  (bind _widgetinteractionleft (`self.WidgetInteractionLeft`))
  (bind (_returnvalue_location_3 _returnvalue_rotation_3) (`KismetMathLibrary.BreakTransform` (`SceneComponent.GetRelativeTransform` (`self.MotionControllerRight`))))
  (bind (_returnvalue_location_4 _returnvalue_rotation_4) (`KismetMathLibrary.BreakTransform` (`SceneComponent.GetRelativeTransform` (`self.MotionControllerLeft`))))
  (bind (_bblockinghit _binitialoverlap _time _distance _location) (`GameplayStatics.BreakHitResult` (`WidgetInteractionComponent.GetLastHitResult` _widgetinteractionright)))
  (bind (_bblockinghit_2 _binitialoverlap_2 _time_2 _distance_2 _location_2) (`GameplayStatics.BreakHitResult` (`WidgetInteractionComponent.GetLastHitResult` _widgetinteractionleft)))
  (if (`OculusXRInputFunctionLibrary.IsHandTrackingEnabled`)
    (`|ExecutionSequence`
      (:`then_0`
        (switch `EOculusXRTrackingConfidence` (`OculusXRInputFunctionLibrary.GetTrackingConfidence` "HandLeft")
          (:`Low`
            (`SceneComponent.SetVisibility` (`self.InteractionSphereLeft`) false false :!label _label))
          (:`High`
            (if (`OculusXRInputFunctionLibrary.IsPointerPoseValid` "HandLeft")
              (`SceneComponent.K2_SetRelativeLocationAndRotation` (`self.WidgetInteractionLeft`) _returnvalue_location _returnvalue_rotation false false)
              (`SceneComponent.SetVisibility` (`self.InteractionSphereLeft`) (`WidgetInteractionComponent.IsOverFocusableWidget` _widgetinteractionleft) false :!label _label_2)
              (if _bblockinghit_2
                (`SceneComponent.K2_SetWorldLocation` (`self.InteractionSphereLeft`) _location_2 false false))
              (else
                (goto _label))))))
      (:`then_1`
        (switch `EOculusXRTrackingConfidence` (`OculusXRInputFunctionLibrary.GetTrackingConfidence` "HandRight")
          (:`Low`
            (`SceneComponent.SetVisibility` (`self.InteractionSphereRight`) false false :!label _label_3))
          (:`High`
            (if (`OculusXRInputFunctionLibrary.IsPointerPoseValid` "HandRight")
              (`SceneComponent.K2_SetRelativeLocationAndRotation` (`self.WidgetInteractionRight`) _returnvalue_location_2 _returnvalue_rotation_2 false false)
              (`SceneComponent.SetVisibility` (`self.InteractionSphereRight`) (`WidgetInteractionComponent.IsOverFocusableWidget` _widgetinteractionright) false :!label _label_4)
              (if _bblockinghit
                (`SceneComponent.K2_SetWorldLocation` (`self.InteractionSphereRight`) _location false false))
              (else
                (goto _label_3)))))))
    (else
      (`|ExecutionSequence`
        (:`then_0`
          (`SceneComponent.K2_SetRelativeLocationAndRotation` (`self.WidgetInteractionLeft`) _returnvalue_location_4 _returnvalue_rotation_4 false false)
          (goto _label_2))
        (:`then_1`
          (`SceneComponent.K2_SetRelativeLocationAndRotation` (`self.WidgetInteractionRight`) _returnvalue_location_3 _returnvalue_rotation_3 false false)
          (goto _label_4))))))

(fn `UserConstructionScript`)