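; BP_ManequinRetarget drives an Unreal mannequin with Oculus XR body tracking on a retarget mesh.
; On BeginPlay it initializes foot grounding, caches the anim Blueprint, binds to the game instance's joint-set change event and starts upper-body tracking.
; Each joint-set change restarts tracking, with foot grounding enabled only for upper body.
; A helper function toggles in-editor animation updates on the mesh's skeletal children.
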(event `self.ReceiveBeginPlay`
  (`parent.ReceiveBeginPlay`)
  ;[1 1 1] We need to initialize the foot grounding component here
  (`/Game/Blueprints/AC_FootGrounding.Initialize` (`self.FootGrounding`) (`self.TargetRetargetMesh`) "foot_r" "foot_l")
  ;[1 1 1] Fetch and store anim blueprint for use later
  (bind _asab_mannequin (cast `/Game/Pawns/UnrealManequin/AB_Mannequin` (`SkeletalMeshComponent.GetAnimInstance` (`self.TargetRetargetMesh`)))
    (:`then`
      (set `self.AnimBlueprint` _asab_mannequin)
      ;[1 1 1] Hook up UI event: When the user selects a new body tracking mode, we need to start body tracking of the new mode
      (bind _asbp_game_instance (cast `/Game/Blueprints/BP_GameInstance` (`GameplayStatics.GetGameInstance`)))
      (add `/Game/Blueprints/BP_GameInstance.BodyJointSetChanged` _asbp_game_instance (delegate `OnFBSChanged`))
      ;[0 1 0.4031] Start the body tracking: Default to Upper Body
      (`self.StartBodyTracking` "UpperBody"))
    (:`CastFailed`
      (`KismetSystemLibrary.PrintString` "Failed to cast to AB_Mannequin"))))

(event `OnFBSChanged`
  (params (OculusXRBodyJointSet :type "EOculusXRBodyJointSet Enum" :default "UpperBody"))
  ;[1 1 1] Hook up UI event: When the user selects a new body tracking mode, we need to start body tracking of the new mode
  (`self.StartBodyTracking` OculusXRBodyJointSet))

(event `StartBodyTracking`
  (params (BodyJointSet :type "EOculusXRBodyJointSet Enum" :default "UpperBody"))
  ;[1 1 1] Start body tracking
  ;;[1 1 1] 2. Enable foot grounding if we are using upper body
  (`/Game/Blueprints/AC_FootGrounding.SetFootGroundingEnabled` (`self.FootGrounding`) (`|EnumEquality` BodyJointSet "UpperBody"))
  ;;[1 1 1] 3. Request body tracking of the new type from the body tracking system
  (`OculusXRMovementFunctionLibrary.StartBodyTrackingByJointSet` BodyJointSet))

(event `self.ReceiveTick`
  (params (DeltaSeconds :type "Float (single-precision)"))
  (`parent.ReceiveTick` DeltaSeconds))

(fn `SetUpdateAnimationInEditor`
  (params (IsEnabled :type Boolean))
  (for _array_element (`SceneComponent.GetChildrenComponents` (`self.TargetRetargetMesh`) true)
    (bind _asskeletal_mesh_component (cast `SkeletalMeshComponent` _array_element))
    (`SkeletalMeshComponent.SetUpdateAnimationInEditor` _asskeletal_mesh_component IsEnabled)))

(fn `UserConstructionScript`)