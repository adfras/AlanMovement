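; Owen character Blueprint that runs OculusXR body tracking alongside face and eye tracking.
; On BeginPlay it initializes foot grounding, caches its animation Blueprint, binds to the game instance's joint-set change event, then starts all tracking, defaulting to upper body.
; Each joint-set change restarts body tracking in the new mode and enables foot grounding only for upper body.
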(event `self.ReceiveBeginPlay`
  (`parent.ReceiveBeginPlay`)
  ;[1 1 1] We need to initialize the foot grounding component here
  (`/Game/Blueprints/AC_FootGrounding.Initialize` (`self.AC_FootGrounding`) (`self.SkeletalMesh`) "RightFoot" "LeftFoot")
  ;[1 1 1] Fetch and store anim blueprint for use later
  (bind _asabp_owen_full_tracking (cast `/Game/Pawns/OwenAnimationNodes/ABP_OwenFullTracking` (`SkeletalMeshComponent.GetAnimInstance` (`self.SkeletalMesh`))))
  (set `self.AnimBlueprint` _asabp_owen_full_tracking)
  ;[1 1 1] Hook up UI event: When the user selects a new body tracking mode, we need to start body tracking of the new mode
  (bind _asbp_game_instance (cast `/Game/Blueprints/BP_GameInstance` (`GameplayStatics.GetGameInstance`)))
  (add `/Game/Blueprints/BP_GameInstance.BodyJointSetChanged` _asbp_game_instance (delegate `OnFBSChanged`))
  ;[0 1 0.4031] Start the body tracking: Default to Upper Body
  (`self.StartBodyTracking` "UpperBody")
  (`OculusXRMovementFunctionLibrary.StartFaceTracking`)
  (`OculusXRMovementFunctionLibrary.StartEyeTracking`))

(event `OnFBSChanged`
  (params (OculusXRBodyJointSet :type "EOculusXRBodyJointSet Enum" :default "UpperBody"))
  ;[1 1 1] Hook up UI event: When the user selects a new body tracking mode, we need to start body tracking of the new mode
  (`self.StartBodyTracking` OculusXRBodyJointSet))

(event `StartBodyTracking`
  (params (BodyJointSet :type "EOculusXRBodyJointSet Enum" :default "UpperBody"))
  ;[1 1 1] Start body tracking
  ;;[1 1 1] 2. Enable foot grounding if we are using upper body
  (`/Game/Blueprints/AC_FootGrounding.SetFootGroundingEnabled` (`self.AC_FootGrounding`) (`|EnumEquality` BodyJointSet "UpperBody"))
  ;;[1 1 1] 3. Request body tracking of the new type from the body tracking system
  (`OculusXRMovementFunctionLibrary.StartBodyTrackingByJointSet` BodyJointSet))

(fn `UserConstructionScript`
  (`parent.UserConstructionScript`))